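; ChargeStation is a charge pad that refills the 2D_Player's SwordLength while something overlaps its HealDetect component.
; BeginPlay caches the player character; overlap begin restarts a Timeline and overlap end stops it, with no check on which actor overlaps.
; Each Timeline update adds a fixed step to SwordLength until it reaches a cap, so the rate follows update frequency, and prints the result for debugging.
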(event `self.ReceiveBeginPlay`
  (bind _as2d_player (cast `/Game/Logan/Player/2D_Player` (`GameplayStatics.GetPlayerCharacter` 0)))
  (set `self.As 2D Player` _as2d_player))

(event `self.Heal detect.OnComponentBeginOverlap`
  (params (OverlappedComponent :type "PrimitiveComponent Object Reference") (OtherActor :type "Actor Object Reference") (OtherComp :type "PrimitiveComponent Object Reference") (OtherBodyIndex :type Integer) (bFromSweep :type Boolean) (SweepResult :type "HitResult Structure (by ref)"))
  (bind _as_2d_player (`self.As 2D Player`))
  (bind _swordlength (`/Game/Logan/Player/2D_Player.SwordLength` _as_2d_player))
  (`Timeline|Timeline` :!via `PlayFromStart` :!label _label
    (:`Update`
      (if (>= _swordlength 10.0)
        (`KismetSystemLibrary.PrintString` "full sword")
        (else
          (bind _output_get (set `/Game/Logan/Player/2D_Player.SwordLength` (+ _swordlength 1.0) _as_2d_player))
          (`KismetSystemLibrary.PrintString` (`KismetStringLibrary.Conv_DoubleToString` _output_get)))))))

(event `self.Heal detect.OnComponentEndOverlap`
  (params (OverlappedComponent :type "PrimitiveComponent Object Reference") (OtherActor :type "Actor Object Reference") (OtherComp :type "PrimitiveComponent Object Reference") (OtherBodyIndex :type Integer))
  (goto _label :!via `Stop`))

(fn `UserConstructionScript`)