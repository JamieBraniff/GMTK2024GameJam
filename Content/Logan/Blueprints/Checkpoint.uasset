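; Checkpoint actor that sets the player's respawn point when touched, in a game using a 2D_Player character.
; On BeginPlay it caches the player character cast to 2D_Player.
; When the player overlaps the Box, a DoOnce writes the Billboard's world location into the player's RespawnPoint, then destroys the checkpoint after a short delay.
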(event `self.ReceiveBeginPlay`
  (bind _as2d_player (cast `/Game/Logan/Player/2D_Player` (`GameplayStatics.GetPlayerCharacter` 0)))
  (set `self.As 2D Player` _as2d_player))

(event `self.ReceiveActorBeginOverlap`
  (params (OtherActor :type "Actor Object Reference")))

(event `self.Box.OnComponentBeginOverlap`
  (params (OverlappedComponent :type "PrimitiveComponent Object Reference") (OtherActor :type "Actor Object Reference") (OtherComp :type "PrimitiveComponent Object Reference") (OtherBodyIndex :type Integer) (bFromSweep :type Boolean) (SweepResult :type "HitResult Structure (by ref)"))
  (if (== OtherActor (`GameplayStatics.GetPlayerCharacter` 0))
    (`/Engine/EditorBlueprintResources/StandardMacros.DoOnce` false
      (:`Completed`
        (set `/Game/Logan/Player/2D_Player.Respawn Point` (`SceneComponent.K2_GetComponentLocation` (`self.Billboard`)) (`self.As 2D Player`))
        (`KismetSystemLibrary.Delay` 0.2)
        (`self.K2_DestroyActor`)))))

(fn `UserConstructionScript`)