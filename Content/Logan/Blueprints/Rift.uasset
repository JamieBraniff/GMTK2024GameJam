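; Rift is a two-way teleporter that moves the 2D_Player between its two sides when Interact is active inside either trigger box.
; Overlap events set range flags for each box, without filtering which actor overlaps.
; A Loop timeline started at BeginPlay polls those flags on update and places the player at the opposite side, slightly offset in Y.
; Each jump starts a cooldown that shrinks both rift visuals, waits, then re-enables travel as they grow back.
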(event `self.ReceiveBeginPlay`
  (bind _as2d_player (cast `/Game/Logan/Player/2D_Player` (`GameplayStatics.GetPlayerCharacter` 0)))
  (set `self.As 2D Player` _as2d_player)
  (`self.Requirements loop`))

(event `Requirements loop`
  (bind (_returnvalue_x _returnvalue_y _returnvalue_z) (`KismetMathLibrary.BreakVector` (`SceneComponent.K2_GetComponentLocation` (`self.Side 1`))))
  (bind (_returnvalue_x_2 _returnvalue_y_2 _returnvalue_z_2) (`KismetMathLibrary.BreakVector` (`SceneComponent.K2_GetComponentLocation` (`self.Side 2`))))
  (`Timeline|loop`
    (:`Update`
      (if (and (`/Game/Logan/Player/2D_Player.Interact?` (`self.As 2D Player`)) (`self.In range 1?`) (`self.CoolDownOver?`))
        (`self.K2_SetActorLocation` (`self.As 2D Player`) (`KismetMathLibrary.MakeVector` _returnvalue_x_2 (+ _returnvalue_y_2 5.0) _returnvalue_z_2) false false)
        (`self.Cooldown`)
        (elif (and (`/Game/Logan/Player/2D_Player.Interact?` (`self.As 2D Player`)) (`self.In range 2?`) (`self.CoolDownOver?`))
          (`self.K2_SetActorLocation` (`self.As 2D Player`) (`KismetMathLibrary.MakeVector` _returnvalue_x (+ _returnvalue_y 5.0) _returnvalue_z) false false)
          (`self.Cooldown`))))))

(event `Cooldown`
  (set `self.CoolDownOver?` false)
  (bind (_direction _newtrack_0) (`Timeline|TL_Shrink` :!via `ReverseFromEnd`)
    (:`Update`
      (bind _returnvalue (`KismetMathLibrary.VLerp` (0.0 0.0 0.0) (0.81431 1.01172 0.81431) _newtrack_0))
      (`SceneComponent.SetRelativeScale3D` (`self.Property`) _returnvalue)
      (`SceneComponent.SetRelativeScale3D` (`self.Property1`) _returnvalue))
    (:`Finished`
      (`KismetSystemLibrary.Delay` 10.0)
      (set `self.CoolDownOver?` true)
      (bind (_direction_2 _newtrack_0_2) (`Timeline|TL_Grow` :!via `PlayFromStart`)
        (:`Update`
          (bind _returnvalue_2 (`KismetMathLibrary.VLerp` (0.0 0.0 0.0) (0.81431 1.01172 0.81431) _newtrack_0_2))
          (`SceneComponent.SetRelativeScale3D` (`self.Property`) _returnvalue_2)
          (`SceneComponent.SetRelativeScale3D` (`self.Property1`) _returnvalue_2))))))

(event `self.Box.OnComponentBeginOverlap`
  (params (OverlappedComponent :type "PrimitiveComponent Object Reference") (OtherActor :type "Actor Object Reference") (OtherComp :type "PrimitiveComponent Object Reference") (OtherBodyIndex :type Integer) (bFromSweep :type Boolean) (SweepResult :type "HitResult Structure (by ref)"))
  (set `self.In range 1?` true))

(event `self.Box.OnComponentEndOverlap`
  (params (OverlappedComponent :type "PrimitiveComponent Object Reference") (OtherActor :type "Actor Object Reference") (OtherComp :type "PrimitiveComponent Object Reference") (OtherBodyIndex :type Integer))
  (set `self.In range 1?` false))

(event `self.Box1.OnComponentBeginOverlap`
  (params (OverlappedComponent :type "PrimitiveComponent Object Reference") (OtherActor :type "Actor Object Reference") (OtherComp :type "PrimitiveComponent Object Reference") (OtherBodyIndex :type Integer) (bFromSweep :type Boolean) (SweepResult :type "HitResult Structure (by ref)"))
  (set `self.In range 2?` true))

(event `self.Box1.OnComponentEndOverlap`
  (params (OverlappedComponent :type "PrimitiveComponent Object Reference") (OtherActor :type "Actor Object Reference") (OtherComp :type "PrimitiveComponent Object Reference") (OtherBodyIndex :type Integer))
  (set `self.In range 2?` false))

(fn `UserConstructionScript`)